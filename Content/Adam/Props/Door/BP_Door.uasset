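; BP_Door is an interactive door prop that swings open and closed when the player presses Interact.
; Overlapping the DoorCollision component enables player input on the actor, and nothing here disables it again.
; IA_Interact plays or reverses the DoorOpenCool timeline based on DoorOpen, and the timeline drives the Door's yaw.
; DoorOpen flips on every timeline Update tick rather than once when the swing finishes.
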(event `self.DoorCollision.OnComponentBeginOverlap`
  (params (OverlappedComponent :type "PrimitiveComponent Object Reference") (OtherActor :type "Actor Object Reference") (OtherComp :type "PrimitiveComponent Object Reference") (OtherBodyIndex :type Integer) (bFromSweep :type Boolean) (SweepResult :type "HitResult Structure (by ref)"))
  (`self.EnableInput` (`GameplayStatics.GetPlayerController` 0)))

(event `EnhancedInput|/Game/Adam/Game/Actions/IA_Interact`
  (params (ActionValue :type Boolean) (ElapsedSeconds :type "Float (double-precision)") (TriggeredSeconds :type "Float (double-precision)") (InputAction :type "InputAction Object Reference" :default "/Game/Adam/Game/Actions/IA_Interact.IA_Interact"))
  (bind _dooropen (`self.doorOpen`))
  (:`Triggered`
    (if _dooropen
      (bind (_direction _newtrack_0) (`Timeline|door open cool` :!via `Reverse` :!label _label)
        (:`Update`
          (set `self.doorOpen` (not _dooropen))
          (`SceneComponent.K2_SetRelativeRotation` (`self.Door`) (`KismetMathLibrary.MakeRotator` 0.0 0.0 _newtrack_0) false false)))
      (else
        (goto _label)))))

(fn `UserConstructionScript`)